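; BP_Test_TPSTurret is a test turret Blueprint that receives and reports its ammo and fire-rate settings.
; Its SetTurretData event stores the incoming values in AmmoCount and FireFrequency, then prints both on screen for debugging.
; It has no firing logic: BeginPlay, overlap and Tick are disabled stubs, and the construction script only calls its parent.
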(event Custom|SetTurretData
  (params (Ammo :type Integer) (Freq :type Float%20%28double-precision%29))
  (bind _output_get (Variables|Default|SetAmmoCount Ammo))
  (bind _output_get_2 (Variables|Default|SetFireFrequency Freq))
  (Development|PrintString (Utilities|String|Append "Ammo: " (Utilities|String|ToString(Integer) _output_get) ", Freq: " (Utilities|String|ToString(Float) _output_get_2)) true true "(R=0.000000,G=0.660000,B=1.000000,A=1.000000)" 5.0))

(event EventBeginPlay
  (|CallParentFunction) ; This node is disabled and will not be called.\nDrag off pins to build functionality.
)

(event Collision|EventActorBeginOverlap
  (params (OtherActor :type Actor%20Object%20Reference))
  (|CallParentFunction OtherActor) ; This node is disabled and will not be called.\nDrag off pins to build functionality.
)

(event EventTick
  (params (DeltaSeconds :type Float%20%28single-precision%29))
  (|CallParentFunction DeltaSeconds) ; This node is disabled and will not be called.\nDrag off pins to build functionality.
)

(fn ConstructionScript
  (|CallParentFunction))